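; BP_Car is a configurable car prop in four body types: hatchback, pickup, station wagon and ambulance.
; The construction script calls ConstructCar, which picks a mesh variation, clean or default material and optional matching foliage mesh.
; FullyRandom randomizes type, variation, color and foliage, while LOCKVALUES suppresses re-randomizing.
; Paint color feeds a dynamic material instance from a palette or manual value, with ambulances using a fixed color.
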(event EventBeginPlay)

(event Collision|EventActorBeginOverlap
  (params (OtherActor :type Actor%20Object%20Reference)))

(event EventTick
  (params (DeltaSeconds :type Float%20%28single-precision%29)))

(fn ConstructionScript
  (CallFunction|ConstructCar (Variables|1.MasterControl|GetRUN_SCRIPT)))

(fn ConstructCar
  (params (RunFunction :type Boolean))
  (bind _carcolors (Variables|4.Colors|GetCarColors))
  (bind _car (Variables|Default|GetCar))
  (bind _foliage (Variables|Default|GetFoliage))
  (if (and RunFunction (not (Variables|1.MasterControl|GetLOCK_VALUES)))
    (Variables|1.MasterControl|SetRUN_SCRIPT false :!label _label)
    (if (Variables|2.RandomControl|GetFullyRandom)
      ;[1 0 0.03529] If fully Random
      (Variables|3.MainControl|SetCarType (Utilities|Select :Index (Math|Random|RandomInteger 4) :Option%200 "NewEnumerator0" :Option%201 "NewEnumerator1" :Option%202 "NewEnumerator2" :Option%203 "NewEnumerator3"))
      (Variables|2.RandomControl|SetRandomColor true)
      (Variables|3.MainControl|SetAllowFoliage (Math|Random|RandomBool)))
    (elif (Variables|1.MasterControl|GetLOCK_VALUES)
      (Variables|1.MasterControl|SetRUN_SCRIPT false)
      (Variables|2.RandomControl|SetFullyRandom false)
      (Variables|2.RandomControl|SetRandomColor false)
      (else
        (goto _label))))
  ;[1 1 1] Set Vehicle Type
  (Variables|Default|SetActiveArray (Utilities|Select :Index (Variables|3.MainControl|GetCarType) :NewEnumerator0 (Variables|Default|GetCarVariationsHatchback) :NewEnumerator1 (Variables|Default|GetCarVariationsPickup) :NewEnumerator2 (Variables|Default|GetCarVariationsWagon) :NewEnumerator3 (Variables|Default|GetCarVariationsAmbulance)))
  (if (Variables|2.RandomControl|GetFullyRandom)
    ;[1 0 0.03529] Set Random Mesh Variation
    (Variables|3.MainControl|SetVehicleVariation (Math|Random|RandomInteger (Utilities|Array|Length (Variables|Default|GetActiveArray)))))
  ;[1 1 1] Set Mesh Variation
  (Components|StaticMesh|SetStaticMesh (Variables|Default|GetCar) (Utilities|Array|Get(acopy) (Variables|Default|GetActiveArray) (Math|Integer|Clamp(Integer) (Variables|3.MainControl|GetVehicleVariation) 0 (- (Utilities|Array|Length (Variables|Default|GetActiveArray)) 1))))
  ;[1 1 1] Create Material Instance
  (bind _returnvalue (Rendering|Material|CreateDynamicMaterialInstance _car 0 (select (Variables|3.MainControl|GetCleanVersion) (Utilities|Select :Index (Variables|3.MainControl|GetCarType) :NewEnumerator0 "/Game/场景/PostDistrict/Materials/Vehicles/MI_Hatchback_Clean.MI_Hatchback_Clean" :NewEnumerator1 "/Game/场景/PostDistrict/Materials/Vehicles/MI_Pickup_Clean.MI_Pickup_Clean" :NewEnumerator2 "/Game/场景/PostDistrict/Materials/Vehicles/MI_Wagon_Clean.MI_Wagon_Clean" :NewEnumerator3 "/Game/场景/PostDistrict/Materials/Vehicles/MI_Ambulance_Clean.MI_Ambulance_Clean") (Utilities|Select :Index (Variables|3.MainControl|GetCarType) :NewEnumerator0 "/Game/场景/PostDistrict/Materials/Vehicles/MI_Hatchback.MI_Hatchback" :NewEnumerator1 "/Game/场景/PostDistrict/Materials/Vehicles/MI_Pickup.MI_Pickup" :NewEnumerator2 "/Game/场景/PostDistrict/Materials/Vehicles/MI_Wagon.MI_Wagon" :NewEnumerator3 "/Game/场景/PostDistrict/Materials/Vehicles/MI_Ambulance.MI_Ambulance")) "None" :!class /Script/Engine.PrimitiveComponent))
  (bind _output_get (Variables|Default|SetCarBodyMatInst _returnvalue))
  (Rendering|Material|SetMaterial _car 0 _output_get)
  (if (Utilities|Enum|Equal(Enum) (Variables|3.MainControl|GetCarType) "NewEnumerator3")
    (Variables|4.Colors|SetActiveCarPaintColor "(R=0.489583,G=0.460799,B=0.397787,A=1.000000)")
    (elif (Variables|1.MasterControl|GetLOCK_VALUES)
      _
      (else
        (Variables|4.Colors|SetActiveCarPaintColor (select (Variables|2.RandomControl|GetRandomColor) (Utilities|Array|Get(acopy) _carcolors (Math|Random|RandomInteger (Utilities|Array|Length _carcolors))) (Variables|4.Colors|GetActiveCarPaintColor))))))
  (Rendering|Material|SetVectorParameterValue (Variables|Default|GetCarBodyMatInst) "AlbedoColor" (Variables|4.Colors|GetActiveCarPaintColor) :!class /Script/Engine.MaterialInstanceDynamic)
  ;[1 1 1] Add Foliage
  (if (Variables|3.MainControl|GetAllowFoliage)
    (Components|StaticMesh|SetStaticMesh _foliage (Utilities|Array|Get(acopy) (Utilities|Select :Index (Variables|3.MainControl|GetCarType) :NewEnumerator0 (Variables|Default|GetHatchbackFol) :NewEnumerator1 (Variables|Default|GetPickupFol) :NewEnumerator2 (Variables|Default|GetWagonFol) :NewEnumerator3 (Variables|Default|GetAmbulanceFol)) (Variables|3.MainControl|GetVehicleVariation)))
    (Rendering|SetVisibility _foliage true false)
    (else
      (Components|DestroyComponent (Variables|Default|GetFoliage)))))