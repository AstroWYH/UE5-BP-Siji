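; Parent building actor that lets each building choose wall type, roof type and wall, wood and footer colors.
; Construction script creates tinted dynamic material instances and assigns them by slot name to static mesh children of Walls and Footer.
; It also swaps the roof material and shows or hides the Lighting component from a baked-lighting flag.
; BeginPlay only caches a reference to the first BP_EnvironmentController found.
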(event EventBeginPlay
  ;[1 1 1] Get Environment Controller Reference
  (bind _outactors (Actor|GetAllActorsOfClass "/Game/场景/PostDistrict/Blueprints/Environment/BP_EnvironmentController.BP_EnvironmentController_C"))
  (Variables|Default|SetControllerRef (Utilities|Array|Get(acopy) _outactors)))

(event Collision|EventActorBeginOverlap
  (params (OtherActor :type Actor%20Object%20Reference)))

(event EventTick
  (params (DeltaSeconds :type Float%20%28single-precision%29)))

(fn ConstructionScript
  (Rendering|SetVisibility (Variables|Default|GetLighting) (Variables|Structure|GetStaticLightMode%28BakedLighting%29) true)
  ;[1 1 1] Color Tweaks
  ;;[1 1 1] Set Exterior Wall Colors
  (bind _returnvalue (Rendering|Material|CreateDynamicMaterialInstance (Utilities|Select :Index (Variables|Walls|GetWallTypes) :NewEnumerator0 "/Game/场景/PostDistrict/Materials/Structure/Outer/MI_WoodenWall.MI_WoodenWall" :NewEnumerator2 "/Game/场景/PostDistrict/Materials/Structure/Outer/MI_BrickWallA.MI_BrickWallA") "None" "None" :!class /Script/Engine.KismetMaterialLibrary))
  (bind _output_get (Variables|Default|SetExternalWallInst _returnvalue))
  (Rendering|Material|SetVectorParameterValue _output_get "AlbedoColor" (Variables|Walls|GetOuterWallColor) :!class /Script/Engine.MaterialInstanceDynamic)
  (for _array_element (Components|GetChildrenComponents (Variables|Default|GetWalls) false)
    (bind _as静态网格体组件 (Utilities|Casting|CastToStaticMeshComponent _array_element))
    (Rendering|Material|SetMaterialbyName _as静态网格体组件 "OuterWoodPanels" (Variables|Default|GetExternalWallInst)))
  ;;[1 1 1] Set Wood Color
  (bind _returnvalue_2 (Rendering|Material|CreateDynamicMaterialInstance "/Game/场景/PostDistrict/Materials/Structure/Outer/MI_OuterWood.MI_OuterWood" "None" "None" :!class /Script/Engine.KismetMaterialLibrary))
  (bind _output_get_2 (Variables|Default|SetExternalWoodInst _returnvalue_2))
  (Rendering|Material|SetVectorParameterValue _output_get_2 "AlbedoColor" (Variables|Walls|GetExternalWoodColor) :!class /Script/Engine.MaterialInstanceDynamic)
  (for _array_element_2 (Components|GetChildrenComponents (Variables|Default|GetWalls) false)
    (bind _as静态网格体组件_2 (Utilities|Casting|CastToStaticMeshComponent _array_element_2))
    (Rendering|Material|SetMaterialbyName _as静态网格体组件_2 "LightWoodTrim" (Variables|Default|GetExternalWoodInst)))
  ;;[1 1 1] Set Footer Color
  (bind _returnvalue_3 (Rendering|Material|CreateDynamicMaterialInstance "/Game/场景/PostDistrict/Materials/Structure/Outer/MI_FooterWall.MI_FooterWall" "None" "None" :!class /Script/Engine.KismetMaterialLibrary))
  (bind _output_get_3 (Variables|Default|SetFooterInst _returnvalue_3))
  (Rendering|Material|SetVectorParameterValue _output_get_3 "AlbedoColor" (Variables|Walls|GetFooterColor) :!class /Script/Engine.MaterialInstanceDynamic)
  (for _array_element_3 (Components|GetChildrenComponents (Variables|Default|GetFooter) false)
    (bind _as静态网格体组件_3 (Utilities|Casting|CastToStaticMeshComponent _array_element_3))
    (Rendering|Material|SetMaterialbyName _as静态网格体组件_3 "Footer" (Variables|Default|GetFooterInst)))
  (for _array_element_4 (Components|GetChildrenComponents (Variables|Default|GetWalls) false)
    (bind _as静态网格体组件_4 (Utilities|Casting|CastToStaticMeshComponent _array_element_4))
    (Rendering|Material|SetMaterialbyName _as静态网格体组件_4 "Footer" (Variables|Default|GetFooterInst)))
  ;[1 1 1] Set Roof Type
  (for _array_element_5 (Components|GetChildrenComponents (Variables|Default|GetWalls) false)
    (bind _as静态网格体组件_5 (Utilities|Casting|CastToStaticMeshComponent _array_element_5))
    (Rendering|Material|SetMaterialbyName _as静态网格体组件_5 "Roof" (Utilities|Select :Index (Variables|Structure|GetRoofTypes) :NewEnumerator0 "/Game/场景/PostDistrict/Materials/Structure/Outer/MI_TileRoof_Hexa.MI_TileRoof_Hexa" :NewEnumerator2 "/Game/场景/PostDistrict/Materials/Structure/Outer/MI_MetalRoof.MI_MetalRoof" :NewEnumerator3 "/Game/场景/PostDistrict/Materials/Structure/Outer/MI_TileRoof_Red.MI_TileRoof_Red"))))