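; Zombie enemy character with a random mesh and facing that wanders, chases and attacks Player_BP.
; Wander and spotted events set walk speed, with a cooldown-gated scream before the chase and its snarl loop.
; Tick sphere-traces ahead while the blackboard reports a sighting, toggling AI focus and attack animation; a socket-to-socket trace applies melee damage.
; It also handles surface-based footsteps, hit reactions, knockback, custom-depth marking and ragdoll death with delayed destroy.
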(event EventBeginPlay
  (bind _outactors (Actor|GetAllActorsOfClass "/Game/所有蓝图/角色/Player_BP.Player_BP_C"))
  (Variables|Default|Set玩家蓝图实例 (Utilities|Array|Get(acopy) _outactors))
  (CallFunction|随机zombie模型)
  (Transformation|SetActorRotation (Math|Rotator|MakeRotator 0.0 0.0 (Math|Random|RandomFloatinRange -1.8e+02 1.8e+02))))

(event Collision|EventActorBeginOverlap
  (params (OtherActor :type Actor%20Object%20Reference)))

(event EventTick
  (params (DeltaSeconds :type Float%20%28single-precision%29)))

(event Custom|随机找点移动
  (if (not (Variables|Default|Get是否死亡))
    (Variables|/Script/Engine.CharacterMovementComponent|SetMaxWalkSpeed (Variables|Character|GetCharacterMovement) 2e+01)
    (Utilities|FlowControl|Sequence
      (:then_0
        (Utilities|IsValid (Variables|Default|Get丧尸追逐音效)
          (:Is%20Valid
            (Components|DestroyComponent (Variables|Default|Get丧尸追逐音效))
            (Variables|Default|Set丧尸追逐音效 0))))
      (:then_1
        (Utilities|FlowControl|DoOnce false
          (:Completed
            (Utilities|Time|SetTimerbyFunctionName 0 "重置尖叫" 15.0)))))))

(event Custom|Reset
  (Utilities|FlowControl|DoOnce false) ; enters at Reset
)

(event Custom|重置尖叫
  (Variables|Default|Set是否可以尖叫 true))

(event Custom|发现玩家要做的事
  (if (Utilities|Enum|Equal(Enum) (Variables|/Game/所有蓝图/角色/Player_BP.Player_BP_C|GetPlayerFunction_State (Variables|Default|Get玩家蓝图实例)) "NewEnumerator7")
    (AI|Components|Blackboard|SetValueasBool (AI|GetBlackboard (AI|GetAIController self)) (Utilities|Name|MakeLiteralName "是否看到玩家") false)
    (elif (not (Variables|Default|Get是否死亡))
      (CallFunction|Reset)
      (Utilities|Time|ClearTimerbyFunctionName 0 "重置尖叫")
      (if (Variables|Default|Get是否可以尖叫)
        (Variables|Default|Set是否可以尖叫 false)
        (Variables|Default|Set正在尖叫 true)
        (bind _returnvalue (Animation|Montage|MontagePlay (Components|SkeletalMesh|GetAnimInstance (Variables|Character|GetMesh)) "/Game/丧尸素材/ZombieAnim/Zombie_Scream_Montage.Zombie_Scream_Montage" 1.0 "MontageLength" 0.0 true))
        (Variables|/Script/Engine.CharacterMovementComponent|SetMaxWalkSpeed (Variables|Character|GetCharacterMovement) 0.0)
        (Utilities|FlowControl|Delay _returnvalue)
        (Variables|Default|Set正在尖叫 false)
        (Variables|/Script/Engine.CharacterMovementComponent|SetMaxWalkSpeed (Variables|Character|GetCharacterMovement) (Math|Random|RandomFloatinRange 4e+02 5e+02) :!label _label)
        (if (not (Variables|Default|Get是否死亡))
          (bind _returnvalue_2 (Audio|SpawnSoundAttached "/Game/丧尸素材/Sounds/Aggressive_Zombie_Snarls_Cue.Aggressive_Zombie_Snarls_Cue" (Variables|Character|GetMesh) "None" "0, 0, 0" "0, 0, 0" "KeepRelativeOffset" false 1.0 1.0 (Math|Random|RandomFloatinRange 0.0 6.0) 0 0))
          (Variables|Default|Set丧尸追逐音效 _returnvalue_2))
        (elif (not (Variables|Default|Get正在尖叫))
          (Utilities|IsValid (Variables|Default|Get丧尸追逐音效)
            (:Is%20Not%20Valid
              (goto _label))))))))

(event EventTick
  (params (DeltaSeconds :type Float%20%28single-precision%29))
  (bind _returnvalue (Transformation|GetActorLocation))
  (bind _self self)
  (bind _mesh (Variables|Character|GetMesh))
  (bind _returnvalue_2 (Components|SkeletalMesh|GetAnimInstance _mesh))
  (bind _returnvalue_3 (AI|GetAIController _self))
  (bind _aszombie_anim (Utilities|Casting|CastToZombie_Anim _returnvalue_2))
  (if (not (Variables|Default|Get是否死亡))
    (if (ScalableFloat|GetValueasBool (AI|GetBlackboard (AI|GetAIController self)) (Utilities|Name|MakeLiteralName "是否看到玩家"))
      (bind (_outhit _returnvalue_4) (Collision|SphereTraceByChannel _returnvalue (+ (* (Transformation|GetActorForwardVector) 1.1e+02) _returnvalue) 1e+02 "TraceTypeQuery5" false 0 "None"))
      (if _returnvalue_4
        (bind _asplayer_bp (Utilities|Casting|CastToPlayer_BP (.HitActor (Collision|BreakHitResult _outhit)))
          (:then
            (if (Variables|/Game/所有蓝图/角色/Player_BP.Player_BP_C|Get是否死亡 _asplayer_bp)
              (Variables|/Game/所有蓝图/Zombie/Zombie_Anim.Zombie_Anim_C|Set是否攻击 _aszombie_anim false :!label _label)
              (CallFunction|更改控制旋转模式 true false)
              (AI|ClearFocus _returnvalue_3)
              (Utilities|Time|ClearTimerbyFunctionName 0 "攻击范围")
              (Variables|Default|SetHitPlayer 0)
              (else
                (Variables|/Game/所有蓝图/Zombie/Zombie_Anim.Zombie_Anim_C|Set是否攻击 _aszombie_anim true)
                (CallFunction|更改控制旋转模式 false true)
                (AI|SetFocus _returnvalue_3 _asplayer_bp))))
          (:CastFailed
            (goto _label)))
        (else
          (goto _label)))
      (else
        (goto _label)))))

(event Custom|右脚脚步声
  (if (not (Variables|Default|Get是否死亡))
    (CallFunction|脚步声判断 (Variables|Default|Get右脚))))

(event Custom|左脚脚步声
  (if (not (Variables|Default|Get是否死亡))
    (CallFunction|脚步声判断 (Variables|Default|Get左脚))))

(event Custom|随机zombie模型
  (Class|SkinnedMeshComponent|SetSkeletalMesh (Variables|Character|GetMesh) (Utilities|Array|Get(acopy) (Variables|Default|Get丧尸模型) (Math|Random|RandomIntegerinRange 0 11)) true))

(event Game|Damage|EventAnyDamage
  (params (Damage :type Float%20%28single-precision%29) (DamageType :type Damage%20Type%20Object%20Reference) (InstigatedBy :type Controller%20Object%20Reference) (DamageCauser :type Actor%20Object%20Reference))
  (bind _aszombie_anim (CallFunction|通信到动画蓝图))
  (bind _丧尸追逐音效 (Variables|Default|Get丧尸追逐音效))
  (bind _output_get (Variables|Default|Set丧尸血量 (- (Variables|Default|Get丧尸血量) Damage)))
  (if (<= _output_get 0.0)
    (Utilities|FlowControl|DoOnce false
      (:Completed
        ;[1 1 1] mesh的碰撞启用要开启查询和物理，否则光开模拟物理没用
        (Physics|SetSimulatePhysics (Variables|Character|GetMesh) true)
        (Variables|/Script/Engine.CharacterMovementComponent|SetMaxWalkSpeed (Variables|Character|GetCharacterMovement) 0.0)
        (Variables|Default|Set是否死亡 true)
        (Collision|SetCollisionEnabled (Variables|Collision|GetCapsuleComponent) "NoCollision")
        (Variables|/Game/所有蓝图/Zombie/Zombie_Anim.Zombie_Anim_C|Set是否攻击 (CallFunction|通信到动画蓝图) false)
        (Utilities|Time|ClearTimerbyFunctionName 0 "攻击范围")
        (Variables|Default|SetHitPlayer 0)
        (Utilities|FlowControl|Sequence
          (:then_0
            (Utilities|IsValid _丧尸追逐音效
              (:Is%20Valid
                (Components|Activation|SetActive _丧尸追逐音效 false false)
                (Components|DestroyComponent _丧尸追逐音效))))
          (:then_1
            (Utilities|FlowControl|Delay 15.0)
            (Actor|DestroyActor)))))
    (elif (not (Variables|/Game/所有蓝图/Zombie/Zombie_Anim.Zombie_Anim_C|Get是否攻击 _aszombie_anim))
      (Variables|/Game/所有蓝图/Zombie/Zombie_Anim.Zombie_Anim_C|Set是否被击中 _aszombie_anim true)
      (Utilities|FlowControl|Delay 0.1)
      (Variables|/Game/所有蓝图/Zombie/Zombie_Anim.Zombie_Anim_C|Set是否被击中 _aszombie_anim false))))

(event Custom|攻击范围
  (bind (_outhit _returnvalue) (Collision|SphereTraceByChannel (Transformation|GetSocketLocation (Variables|Character|GetMesh) (Variables|Default|Get攻击检测起始骨骼)) (Transformation|GetSocketLocation (Variables|Character|GetMesh) (Variables|Default|Get攻击检测终点骨骼)) 25.0 "TraceTypeQuery5" false 0 "None"))
  (if _returnvalue
    (if (!= (Variables|Default|GetHitPlayer) (.HitActor (Collision|BreakHitResult _outhit)))
      (bind _asplayer_bp (Utilities|Casting|CastToPlayer_BP (.HitActor (Collision|BreakHitResult _outhit))))
      (Variables|Default|SetHitPlayer (.HitActor (Collision|BreakHitResult _outhit)))
      (Game|Damage|ApplyDamage _asplayer_bp 1e+01 0 0)
      (Effects|SpawnEmitteratLocation "/Game/粒子特效/Effects1/SmokeBuilder/Particles/P_SmokePuff1b.P_SmokePuff1b" (.Location (Collision|BreakHitResult _outhit)) (Math|Conversions|RotationFromXVector (.ImpactNormal (Collision|BreakHitResult _outhit))) "0.100000,0.100000,0.100000"))))

(event Custom|开启Zombie标记
  (Rendering|SetRenderCustomDepth (Variables|Character|GetMesh) true))

(event Custom|被击退
  (Audio|PlaySound2D "/Game/音效/Punch/punch_general_body_impact_01_Cue.punch_general_body_impact_01_Cue" 1.0 1.0 0.0 0 0)
  (Animation|Montage|PlayMontage (Variables|Character|GetMesh) "/Game/丧尸素材/近战动画/Zombie_Chase_1_KnockBack_Chase_Montage.Zombie_Chase_1_KnockBack_Chase_Montage"))

(fn ConstructionScript)

(fn 更改控制旋转模式
  (params (将旋转朝向运动 :type Boolean) (使用控制器旋转Yaw :type Boolean))
  (Variables|/Script/Engine.CharacterMovementComponent|SetbOrientRotationToMovement (Variables|Character|GetCharacterMovement) 将旋转朝向运动)
  (Variables|Default|SetbUseControllerRotationYaw 使用控制器旋转Yaw))

(fn 通信到动画蓝图
  (bind _aszombie_anim (Utilities|Casting|CastToZombie_Anim (Components|SkeletalMesh|GetAnimInstance (Variables|Character|GetMesh))))
  (return _aszombie_anim))

(fn 脚步声判断
  (params (目标 :type Scene%20Component%20Object%20Reference))
  (bind _returnvalue (Transformation|GetWorldLocation 目标))
  (bind (_outhit _returnvalue_2) (Collision|LineTraceByChannel _returnvalue (- _returnvalue "0, 0,50.000000") "TraceTypeQuery3" false 0 "None"))
  (if _returnvalue_2
    (switch Utilities|FlowControl|Switch|SwitchonEPhysicalSurface (Collision|GetSurfaceType _outhit)
      (:SurfaceType_Default
        (Audio|PlaySoundatLocation "/Game/音效/FootStep/footstep_dirt_walk_run_04_Cue.footstep_dirt_walk_run_04_Cue" (.Location (Collision|BreakHitResult _outhit)) "0, 0, 0" 1.0 1.0 0.0 0 0 0))
      (:SurfaceType1
        (Audio|PlaySoundatLocation "/Game/音效/FootstepSound/Sounds/WaveFiles/Footsteps_Mono/Male/Metal/metal_1_Cue.metal_1_Cue" (.Location (Collision|BreakHitResult _outhit)) "0, 0, 0" 1.0 1.0 0.0 0 0 0))
      (:SurfaceType2
        (Audio|PlaySoundatLocation "/Game/音效/FootStep/footstep_dirt_walk_run_04_Cue.footstep_dirt_walk_run_04_Cue" (.Location (Collision|BreakHitResult _outhit)) "0, 0, 0" 1.0 1.0 0.0 0 0 0))
      (:SurfaceType3
        (Audio|PlaySoundatLocation "/Game/音效/FootstepSound/Sounds/WaveFiles/Footsteps_Mono/Male/Concrete/concrete_1_Cue.concrete_1_Cue" (.Location (Collision|BreakHitResult _outhit)) "0, 0, 0" 1.0 1.0 0.0 0 0 0))
      (:SurfaceType4
        (Audio|PlaySoundatLocation "/Game/音效/Wood/footstep_wood_run_01_Cue.footstep_wood_run_01_Cue" (.Location (Collision|BreakHitResult _outhit)) "0, 0, 0" 1.0 1.0 0.0 0 0 0))
      (:SurfaceType5
        (Audio|PlaySoundatLocation "/Game/音效/FootstepSound/Sounds/WaveFiles/Footsteps_Mono/Male/Concrete/concrete_1_Cue.concrete_1_Cue" (.Location (Collision|BreakHitResult _outhit)) "0, 0, 0" 1.0 1.0 0.0 0 0 0))
      (:SurfaceType6
        (Audio|PlaySoundatLocation "/Game/音效/Grass/footstep_grass_run_01_Cue.footstep_grass_run_01_Cue" (.Location (Collision|BreakHitResult _outhit)) "0, 0, 0" 1.0 1.0 0.0 0 0 0)))))