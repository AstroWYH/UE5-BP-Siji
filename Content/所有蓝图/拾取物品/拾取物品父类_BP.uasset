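; 拾取物品父类_BP is the pickup item parent Blueprint, handling collection by the player and highlighting.
; On BeginPlay it caches the first Player_BP actor.
; 拾取物品 passes PickUpStruct to that player to play the pickup animation, then destroys the item after a short delay matching the hand reach.
; Two events toggle Render Custom Depth on the 拾取模型 mesh to switch the highlight on and off.
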(event EventBeginPlay
  (bind _outactors (Actor|GetAllActorsOfClass "/Game/所有蓝图/角色/Player_BP.Player_BP_C"))
  (Variables|Default|Set角色蓝图实例 (Utilities|Array|Get(acopy) _outactors)))

(event Collision|EventActorBeginOverlap
  (params (OtherActor :type Actor%20Object%20Reference)))

(event EventTick
  (params (DeltaSeconds :type Float%20%28single-precision%29)))

(event Event拾取物品
  (Default|获取拾取信息并播放拾取动画 (Variables|Default|Get角色蓝图实例) (Variables|Default|GetPickUp_Struct))
  ;[1 1 1] 手伸过去的0.4s，让其销毁自己
  (Utilities|FlowControl|Delay 0.4)
  ;[1 1 1] 被拾取的物品销毁
  (Actor|DestroyActor))

(event Event开启高亮显示
  (Rendering|SetRenderCustomDepth (Variables|Default|Get拾取模型) true))

(event Event关闭高亮显示
  (Rendering|SetRenderCustomDepth (Variables|Default|Get拾取模型) false))

(fn ConstructionScript)