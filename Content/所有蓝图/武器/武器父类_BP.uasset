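; Weapon base Blueprint that handles firing, recoil, reloading and cleanup for the player's guns.
; Full-auto fire repeats on a looping timer, each shot spawning a bullet, muzzle effects and ejected shells with collision sounds, while an empty gun dry-fires and stops the player shooting.
; A timeline applies pitch and random yaw recoil, then reverses to recover pitch.
; Reload events move a separate magazine actor between weapon and hand sockets, then refill ammo.
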(event EventBeginPlay
  (Utilities|FlowControl|Sequence
    (:then_0
      (bind _outactors (Actor|GetAllActorsOfClass "/Game/所有蓝图/角色/Player_BP.Player_BP_C"))
      (Variables|Default|Set角色蓝图实例 (Utilities|Array|Get(acopy) _outactors)))
    (:then_1
      (bind _returnvalue (Game|SpawnActorfromClass (Variables|Default|Get弹夹) (Math|Transform|MakeTransform "0, 0, 0") "Undefined" 0 0))
      (bind _output_get (Variables|Default|Set弹夹引用 _returnvalue))
      (Transformation|AttachComponentToComponent _output_get (Variables|Default|Get武器模型) "Gun_magazinesocket" "SnapToTarget" "SnapToTarget" "SnapToTarget" true))))

(event Collision|EventActorBeginOverlap
  (params (OtherActor :type Actor%20Object%20Reference)))

(event EventTick
  (params (DeltaSeconds :type Float%20%28single-precision%29)))

(event Custom|停止射击
  (Utilities|Time|ClearandInvalidateTimerbyHandle (stale Custom|开始射击 _returnvalue)))

(event Custom|射击中
  (bind _武器模型 (Variables|Default|Get武器模型))
  (bind _arrow (Variables|Default|GetArrow))
  (bind _武器模型_2 (Variables|Default|Get武器模型))
  (bind _returnvalue (Transformation|GetSocketTransform _武器模型 "Gun_Muzzle" "RTS_World"))
  (bind _returnvalue_2 (Transformation|GetWorldTransform _arrow))
  (bind _returnvalue_3 (Transformation|GetSocketTransform _武器模型_2 "Gun_Muzzle" "RTS_World"))
  (if (<= (Variables|Default|Get子弹数量) 0)
    (Utilities|FlowControl|DoOnce false :!label _label
      (:Completed
        (Audio|PlaySoundatLocation "/Game/武器素材/Rifles/gun_rifle_dry_fire_01_Cue.gun_rifle_dry_fire_01_Cue" (Transformation|GetActorLocation) "0, 0, 0" 1.0 1.0 0.0 0 0 0)
        (Default|停止射击 (Variables|Default|Get角色蓝图实例))))
    (else
      (Utilities|FlowControl|Sequence
        (:then_0
          (Game|SpawnActorfromClass (Variables|Default|Get生成的子弹) (Math|Transform|MakeTransform (.location _returnvalue_3) (.rotation _returnvalue_3) "0.200000,0.200000,0.200000") "Undefined" 0 0)
          ;[1 1 1] 弹夹纷飞
          (bind _returnvalue_4 (Effects|SpawnEmitteratLocation "/Game/粒子特效/Weapons/Effects/ParticleSystems/Ammo_Shell_Reject2.Ammo_Shell_Reject2" (.location _returnvalue_2) (.rotation _returnvalue_2)))
          (Utilities|FlowControl|Sequence
            (:then_0
              ;[1 1 1] 弹壳落地时触发
              (EventDispatchers|AssignOnParticleCollide _returnvalue_4 (delegate Custom|空弹壳碰撞))
              (bind _counter (Utilities|FlowControl|DoN 3 :!label _label_2)
                (:Exit
                  (if (== _counter 3)
                    (Audio|PlaySoundatLocation "/Game/武器素材/Rifles/Shells/S_Shell_end_01_Cue.S_Shell_end_01_Cue" (stale Custom|空弹壳碰撞 Location) "0, 0, 0" 1.0 1.0 0.0 0 0 0)
                    (Utilities|FlowControl|Delay 0.5)
                    (goto _label_2 Reset)
                    (else
                      (Audio|PlaySoundatLocation "/Game/武器素材/Rifles/Shells/S_Shell_hit_01_Cue.S_Shell_hit_01_Cue" (stale Custom|空弹壳碰撞 Location) "0, 0, 0" 1.0 1.0 0.0 0 0 0))))))
            (:then_1
              ;[1 1 1] 枪口冒烟
              (Effects|SpawnEmitteratLocation "/Game/粒子特效/M4A4_Animated/VFX/Particle_Systems/Muzzle_01.Muzzle_01" (.location _returnvalue) (.rotation _returnvalue) "0.400000,0.400000,0.400000")
              (Components|Animation|PlayAnimation (Variables|Default|Get武器模型) (Variables|Default|Get武器动画) false)
              (CallFunction|后坐力)
              (Math|Integer|DecrementInt (Variables|Default|Get子弹数量)))))
        (:then_1
          (goto _label Reset))))))

(event Custom|空弹壳碰撞
  (params (EventName :type Name) (EmitterTime :type Float%20%28single-precision%29) (ParticleTime :type Integer) (Location :type Vector) (Velocity :type Vector) (Direction :type Vector) (Normal :type Vector) (BoneName :type Name) (PhysMat :type Physical%20Material%20Object%20Reference))
  ;[1 1 1] 弹壳落地时触发
)

(event Custom|开始射击
  (CallFunction|射击中)
  (if (Variables|Default|Get是否全自动)
    (bind _returnvalue (Utilities|Time|SetTimerbyEvent (delegate Custom|射击中) (Variables|Default|Get射速) true))
    (else
      ;[1 1 1] 延迟0.1s，让半自动时，有时间播一下开枪抖动的动画
      (Utilities|FlowControl|Delay 0.1)
      (Default|停止射击 (Variables|Default|Get角色蓝图实例)))))

(event Custom|后坐力回弹
  (bind _returnvalue (Game|Player|GetPlayerPawn 0))
  (bind _后坐力yaw (Variables|Default|Get后坐力Yaw))
  (bind (_direction _新建轨道_0) (Timeline|时间轴_0 Reverse)
    (:Update
      (switch Utilities|FlowControl|Switch|SwitchonETimelineDirection _direction
        (:Forward
          (Pawn|Input|AddControllerPitchInput _returnvalue (Math|Float|Lerp 0.0 (Variables|Default|Get后坐力Pitch) _新建轨道_0))
          (Pawn|Input|AddControllerYawInput _returnvalue (Math|Random|RandomFloatinRange (* _后坐力yaw -1.0) _后坐力yaw)))
        (:Backward
          (Pawn|Input|AddControllerPitchInput (Game|Player|GetPlayerPawn 0) (* (Math|Float|Lerp 0.0 (Variables|Default|Get后坐力Pitch) _新建轨道_0) -1.0)))))
    (:Finished
      (CallFunction|后坐力回弹))))

(event Custom|后坐力
  (bind _returnvalue (Game|Player|GetPlayerPawn 0))
  (bind _后坐力yaw (Variables|Default|Get后坐力Yaw))
  (bind (_direction _新建轨道_0) (Timeline|时间轴_0 PlayFromStart)
    (:Update
      (switch Utilities|FlowControl|Switch|SwitchonETimelineDirection _direction
        (:Forward
          (Pawn|Input|AddControllerPitchInput _returnvalue (Math|Float|Lerp 0.0 (Variables|Default|Get后坐力Pitch) _新建轨道_0))
          (Pawn|Input|AddControllerYawInput _returnvalue (Math|Random|RandomFloatinRange (* _后坐力yaw -1.0) _后坐力yaw)))
        (:Backward
          (Pawn|Input|AddControllerPitchInput (Game|Player|GetPlayerPawn 0) (* (Math|Float|Lerp 0.0 (Variables|Default|Get后坐力Pitch) _新建轨道_0) -1.0)))))
    (:Finished
      (CallFunction|后坐力回弹))))

(event Custom|换弹结束
  (Transformation|AttachComponentToComponent (Variables|Default|Get弹夹引用) (Variables|Default|Get武器模型) "Gun_magazinesocket" "SnapToTarget" "SnapToTarget" "SnapToTarget" true)
  (Variables|Default|Set子弹数量 (Variables|Default|Get子弹总数量)))

(event Custom|拔下弹夹
  (Transformation|AttachComponentToComponent (Variables|Default|Get弹夹引用) (Variables|/Script/Engine.Character|GetMesh (Variables|Default|Get角色蓝图实例)) "换弹" "KeepRelative" "KeepRelative" "KeepRelative" true)
  ;[1 1 1] 把弹夹拔时，再让其跟手一销毁，然后再掉地上
  (Utilities|FlowControl|Delay 0.2)
  (bind _as弹夹父类_bp (Utilities|Casting|CastTo弹夹父类_BP (Variables|Default|Get弹夹引用)))
  (Default|弹夹分离 _as弹夹父类_bp))

(event Custom|生成新弹夹
  (bind _returnvalue (Game|SpawnActorfromClass (Variables|Default|Get弹夹) (Math|Transform|MakeTransform "0, 0, 0") "Undefined" 0 0))
  (Variables|Default|Set弹夹引用 _returnvalue)
  (Transformation|AttachComponentToComponent (Variables|Default|Get弹夹引用) (Variables|/Script/Engine.Character|GetMesh (Variables|Default|Get角色蓝图实例)) "换弹" "SnapToTarget" "SnapToTarget" "SnapToTarget" true)
  (Math|Integer|DecrementInt (Variables|Default|Get弹夹数量)))

(event Custom|自毁
  (Actor|DestroyActor)
  (Actor|DestroyActor (Variables|Default|Get弹夹引用)))

(event Custom|开启物理模拟
  (Physics|SetSimulatePhysics (Variables|Default|Get武器模型) true))

(fn ConstructionScript)