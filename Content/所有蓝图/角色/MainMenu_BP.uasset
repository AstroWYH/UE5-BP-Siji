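; MainMenu_BP is the main menu character whose outfit can be switched and saved.
; Its 切换服装 (switch outfit) event applies the chosen skeletal mesh to Mesh without reinitializing the pose.
; It then loads or creates the ClothSaveGame in slot "cloth", writes the mesh to ClothMesh and saves.
; Nothing here restores the saved outfit on BeginPlay.
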(event Custom|切换服装
  (params (选择的模型 :type Skeletal%20Mesh%20Object%20Reference))
  (bind _output_get (Variables|Default|Set选择的模型 选择的模型))
  (Class|SkinnedMeshComponent|SetSkeletalMesh (Variables|Character|GetMesh) _output_get false)
  (SaveGame|DoesSaveGameExist "cloth")
  (if true
    (bind _returnvalue (SaveGame|LoadGamefromSlot "cloth"))
    (bind _ascloth_save_game (Utilities|Casting|CastToClothSaveGame _returnvalue))
    (Variables|Default|SetClothSaveGame _ascloth_save_game)
    (else
      (bind _returnvalue_2 (SaveGame|CreateSaveGameObject "/Game/所有蓝图/角色/ClothSaveGame.ClothSaveGame_C"))
      (Variables|Default|SetClothSaveGame _returnvalue_2)))
  (Variables|/Game/所有蓝图/角色/ClothSaveGame.ClothSaveGame_C|SetClothMesh (Variables|Default|GetClothSaveGame) (Variables|Default|Get选择的模型))
  (SaveGame|SaveGametoSlot (Variables|Default|GetClothSaveGame) "cloth"))

(event EventBeginPlay)

(event Collision|EventActorBeginOverlap
  (params (OtherActor :type Actor%20Object%20Reference)))

(event EventTick
  (params (DeltaSeconds :type Float%20%28single-precision%29)))

(fn ConstructionScript)